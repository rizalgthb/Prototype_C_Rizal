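; BP_SwatXSpawner is a spawner actor that creates BP_SwatX enemies at its own location and rotation.
; SpawnSwatX spawns a given count at once in a loop, adjusting for collisions but always spawning.
; BatchSpawnSwatx repeats SpawnSwatX in timed waves, using a Delay loop until the batch count runs out.
; BeginPlay is empty and the sample calls are unwired, so spawning relies on outside callers.
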(event `self.ReceiveBeginPlay`)

(event `SpawnSwatX`
  (params (SpawnEnemyCount :type Integer))
  (set `self.SpawnEnemyCount` SpawnEnemyCount)
  (while (> (`self.SpawnEnemyCount`) 0)
    (`|SpawnActorFromClass` "/Game/Enemy/SwatX/Blueprint/BP_SwatX.BP_SwatX_C" (`KismetMathLibrary.MakeTransform` (`self.K2_GetActorLocation`) (`self.K2_GetActorRotation`)) "AdjustIfPossibleButAlwaysSpawn" "MultiplyWithRoot" null null)
    (set `self.SpawnEnemyCount` (- (`self.SpawnEnemyCount`) 1))))

(event `BatchSpawnSwatx`
  (params (BatchSpawnCount :type Integer) (PerbatchEnemySpawn :type Integer) (Interval :type "Float (double-precision)"))
  (set `self.BatchSpawnCount` BatchSpawnCount)
  (`self.SpawnSwatX` PerbatchEnemySpawn :!label _label)
  (set `self.BatchSpawnCount` (- (`self.BatchSpawnCount`) 1))
  (`KismetSystemLibrary.Delay` Interval)
  (if (> (`self.BatchSpawnCount`) 0)
    (goto _label)))

(fn `UserConstructionScript`)