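; BP_SwatX is an enemy that patrols random reachable points and attacks BP_Ember on sight through PawnSensing.
; Each sighting starts an AIMoveTo chase, turns it toward the player and fires a montage-driven muzzle line trace, throttled by a DoOnce reset after the weapon's fire rate.
; The Weapon data supplies mesh, range and damage.
; Lethal damage ragdolls it and drops BP_Ammo; debug health text and trace lines are drawn.
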(event `self.ReceiveBeginPlay`
  (`self.Patrol`))

(event `self.ReceiveAnyDamage`
  (params (Damage :type "Float (single-precision)") (DamageType :type "DamageType Object Reference") (InstigatedBy :type "Controller Object Reference") (DamageCauser :type "Actor Object Reference"))
  (if (not (`self.IsDeath`))
    (set `self.Health` (- (`self.Health`) Damage))
    (if (<= (`self.Health`) 0)
      (set `self.IsDeath` true)
      (`PrimitiveComponent.SetSimulatePhysics` (`self.Mesh`) true)
      (`|SpawnActorFromClass` "/Game/CollectibleItem/BP_Ammo.BP_Ammo_C" (`KismetMathLibrary.MakeTransform` (`self.K2_GetActorLocation`)) "Undefined" "MultiplyWithRoot" null null))))

(event `self.ReceiveTick`
  (params (DeltaSeconds :type "Float (single-precision)"))
  (`KismetSystemLibrary.PrintString` (`KismetStringLibrary.Concat_StrStr` "Enemy Health:" (`KismetStringLibrary.Conv_IntToString` (`self.Health`))) true true (struct :`G` 0.66 :`B` 1.0 :`A` 1.0) 0.001))

(event `Patrol`
  (if (not (`self.IsDeath`))
    (`|AIMoveTo` self (`NavigationSystemV1.K2_GetRandomReachablePointInRadius` (`self.K2_GetActorLocation`) 1500.0 null null) null
      (:`OnSuccess`
        _)
      (:`OnFail`
        _))
    (if (not (`self.IsChasingPlayer`))
      (`self.Patrol`))))

(event `self.PawnSensing.OnSeePawn`
  (params (Pawn :type "Pawn Object Reference"))
  (bind _asbp_ember (cast `/Game/Characters/Player/Ember/BP_Ember` Pawn))
  (set `self.IsChasingPlayer` true)
  (`self.ChasePlayer` _asbp_ember))

(event `ChasePlayer`
  (params (Player :type "/Game/Characters/Player/Ember/BP_Ember Object Reference"))
  (if (not (`self.IsDeath`))
    (`|AIMoveTo` self (0.0 0.0 0.0) Player 1000.0
      (:`then`
        _)
      (:`OnSuccess`
        (set `self.IsChasingPlayer` false :!label _label))
      (:`OnFail`
        (goto _label)))
    (`self.K2_SetActorRotation` (`KismetMathLibrary.FindLookAtRotation` (`self.K2_GetActorLocation`) (`self.K2_GetActorLocation` Player)))
    (`self.Shoot`)))

(event `Shoot`
  (bind _returnvalue (`SceneComponent.GetSocketLocation` (`self.EnemyWeaponMesh`) "MuzzleSocket"))
  (`|ExecutionSequence`
    (:`then_0`
      (`/Engine/EditorBlueprintResources/StandardMacros.DoOnce` false :!label _label_2
        (:`Completed`
          (`|PlayMontage` (`self.Mesh`) "/Game/Enemy/SwatX/Animation/AM_Shoot.AM_Shoot" 0.5
            (:`then`
              (bind _outhit (`KismetSystemLibrary.LineTraceSingle` :`Start` _returnvalue :`End` (+ _returnvalue (* (`KismetMathLibrary.GetForwardVector` (`self.K2_GetActorRotation`)) (`/Game/weapon/Data/BP_DatasetWeapon.FireRange` (`self.Weapon`)))) :`TraceChannel` "TraceTypeQuery1" :`DrawDebugType` "ForDuration" :`DrawTime` 1.0))
              (bind _asbp_ember (cast `/Game/Characters/Player/Ember/BP_Ember` (`.HitActor` (`GameplayStatics.BreakHitResult` _outhit))))
              (`GameplayStatics.ApplyDamage` _asbp_ember (`/Game/weapon/Data/BP_DatasetWeapon.Damage` (`self.Weapon`)))
              (if (`/Game/Characters/Player/Ember/BP_Ember.IsDeath` _asbp_ember)
                (`self.Patrol`)))))))
    (:`then_1`
      (`KismetSystemLibrary.Delay` (`/Game/weapon/Data/BP_DatasetWeapon.FireRate` (`self.Weapon`)))
      (goto _label_2 :!via `Reset`))))

(fn `UserConstructionScript`
  (`SkeletalMeshComponent.SetSkeletalMeshAsset` (`self.EnemyWeaponMesh`) (`/Game/weapon/Data/BP_DatasetWeapon.Mesh` (`self.Weapon`))))