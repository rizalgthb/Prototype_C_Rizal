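; BP_SwatX is a SWAT enemy that takes damage and dies into a ragdoll.
; Any damage lowers Health until it reaches zero, then sets IsDeath and turns on physics simulation on the mesh, ignoring further hits.
; The construction script applies the mesh from its Weapon data to the weapon component, and Tick prints the current health on screen for debugging.
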(event `self.ReceiveAnyDamage`
  (params (Damage :type "Float (single-precision)") (DamageType :type "DamageType Object Reference") (InstigatedBy :type "Controller Object Reference") (DamageCauser :type "Actor Object Reference"))
  (if (not (`self.IsDeath`))
    (set `self.Health` (- (`self.Health`) Damage))
    (if (<= (`self.Health`) 0)
      (set `self.IsDeath` true)
      (`PrimitiveComponent.SetSimulatePhysics` (`self.Mesh`) true))))

(event `self.ReceiveTick`
  (params (DeltaSeconds :type "Float (single-precision)"))
  (`KismetSystemLibrary.PrintString` (`KismetStringLibrary.Concat_StrStr` "Enemy Health:" (`KismetStringLibrary.Conv_IntToString` (`self.Health`))) true true (struct :`G` 0.66 :`B` 1.0 :`A` 1.0) 0.001))

(fn `UserConstructionScript`
  (`SkeletalMeshComponent.SetSkeletalMeshAsset` (`self.EnemyWeaponMesh`) (`/Game/weapon/Data/BP_DatasetWeapon.Mesh` (`self.Weapon`))))